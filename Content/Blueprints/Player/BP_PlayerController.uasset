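; Player controller that manages switching between the HUD and an escape menu, and provides game pause and unpause events.
; On BeginPlay it waits briefly, takes the HUD from the controlled pawn, then creates the escape menu hidden in the viewport.
; Escape toggles which of the two widgets is visible, without pausing.
; Separate PauseGame and UnPauseGame events set the pause state and switch between UI-only and game-only input.
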(event `self.ReceiveBeginPlay`
  (`KismetSystemLibrary.Delay` 0.0)
  (bind _asbp_player (cast `` (`self.K2_GetPawn`)))
  (set `self.HUD` (`/Game/Blueprints/Player/BP_PlayerController.W_HUD` _asbp_player))
  (bind _returnvalue (`|CreateWidget` null self))
  (bind _output_get (set `self.EscapeMenu` _returnvalue))
  (`Widget.SetVisibility` _output_get "Hidden")
  (`UserWidget.AddToViewport` _returnvalue 0))

(event `Key|Escape`
  (params (Key :type "Key Structure"))
  (:`Pressed`
    (`self.ShowHideUI`)))

(event `Pause Game`
  (`GameplayStatics.SetGamePaused` true)
  (`WidgetBlueprintLibrary.SetInputMode_UIOnlyEx` self null))

(event `ShowHideUI`
  (if (`Widget.IsVisible` (`self.HUD`))
    (`Widget.SetVisibility` (`self.HUD`) "Hidden")
    (`Widget.SetVisibility` (`self.EscapeMenu`) "Visible")
    (else
      (`Widget.SetVisibility` (`self.HUD`) "Visible")
      (`Widget.SetVisibility` (`self.EscapeMenu`) "Hidden"))))

(event `UnPauseGame`
  (`GameplayStatics.SetGamePaused` false)
  (`WidgetBlueprintLibrary.SetInputMode_GameOnly` self))

(fn `UserConstructionScript`)