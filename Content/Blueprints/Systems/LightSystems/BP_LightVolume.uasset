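; BP_LightVolume is a light area that raises BP_Player's lighting while the player is inside its mesh with clear line of sight.
; Overlapping the mesh starts a fast looping timer that line-traces on Visibility from the volume to the player.
; Unblocked traces add delta-scaled lighting, while flags limit the player's light-count increments and decrements to changes in visibility.
; Leaving clears the timer and decrements the count unless already removed.
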(event `Fire Ray Cast`
  (bind _player (`self.Player`))
  (bind _player_2 (`self.Player`)
    (:`then`
      (bind (_outhit _returnvalue) (`KismetSystemLibrary.LineTraceSingle` (`self.K2_GetActorLocation`) (`self.K2_GetActorLocation` _player_2) "TraceTypeQuery1"))
      (if _returnvalue
        (if (not (`self.wasLightRemoved`))
          (set `self.wasLightRemoved` true)
          (`/Game/Blueprints/Player/BP_Player.Decrease Num Lights` _player)
          (set `self.wasLightAdded` false))
        (else
          (`/Game/Blueprints/Player/BP_Player.Add Lighting` _player (* (`GameplayStatics.GetWorldDeltaSeconds`) (`self.LightIncreaseRate`)))
          (if (not (`self.wasLightAdded`))
            (set `self.wasLightAdded` true)
            (`/Game/Blueprints/Player/BP_Player.Increase Num Lights` _player)
            (set `self.wasLightRemoved` false)))))
    (:`else`)))

(event `self.StaticMesh.OnComponentBeginOverlap`
  (params (OverlappedComponent :type "PrimitiveComponent Object Reference") (OtherActor :type "Actor Object Reference") (OtherComp :type "PrimitiveComponent Object Reference") (OtherBodyIndex :type Integer) (bFromSweep :type Boolean) (SweepResult :type "HitResult Structure (by ref)"))
  (bind _asbp_player (cast `/Game/Blueprints/Player/BP_Player` OtherActor))
  (set `self.Player` _asbp_player)
  (bind _returnvalue (`KismetSystemLibrary.K2_SetTimerDelegate` (`|CreateDelegate` :!event `Fire Ray Cast`) 0.015 true))
  (set `self.T_RaycastH` _returnvalue)
  (set `self.wasLightRemoved` false)
  (set `self.wasLightAdded` false))

(event `self.StaticMesh.OnComponentEndOverlap`
  (params (OverlappedComponent :type "PrimitiveComponent Object Reference") (OtherActor :type "Actor Object Reference") (OtherComp :type "PrimitiveComponent Object Reference") (OtherBodyIndex :type Integer))
  (cast `/Game/Blueprints/Player/BP_Player` OtherActor)
  (`KismetSystemLibrary.K2_ClearAndInvalidateTimerHandle` (`self.T_RaycastH`))
  (if (not (`self.wasLightRemoved`))
    (`/Game/Blueprints/Player/BP_Player.Decrease Num Lights` (`self.Player`))))

(fn `UserConstructionScript`)