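; Extraction zone actor that checks whether a player entering it carries the objective.
; On box overlap it casts to BP_Player, reads GetHasObjective and sets the objective HUD text to a white success message or a red reminder to get the item.
; It only updates text; no level end or travel happens here.
; The construction script raises the box by its Z extent so it sits on the actor origin.
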(event `self.Box.OnComponentBeginOverlap`
  (params (OverlappedComponent :type "PrimitiveComponent Object Reference") (OtherActor :type "Actor Object Reference") (OtherComp :type "PrimitiveComponent Object Reference") (OtherBodyIndex :type Integer) (bFromSweep :type Boolean) (SweepResult :type "HitResult Structure (by ref)"))
  (bind _asbp_player (cast `/Game/Blueprints/Player/BP_Player` OtherActor))
  (if (`/Game/Blueprints/Player/BP_Player.GetHasObjective` _asbp_player)
    (bind _wbp_objectiveui (`/Game/Blueprints/UMG/WBP_HUD.WBP_ObjectiveUI` (`/Game/Blueprints/Player/BP_Player.W_HUD` _asbp_player)))
    (`/Game/Blueprints/UMG/WBP_ObjectiveUI.Set Objective Text` _wbp_objectiveui "Congratulations!!! Time to head home" (struct :`R` 1.0 :`G` 1.0 :`B` 1.0 :`A` 1.0))
    (else
      (`/Game/Blueprints/UMG/WBP_ObjectiveUI.Set Objective Text` _wbp_objectiveui "GET THE THING DUMBO" (struct :`R` 1.0 :`A` 1.0)))))

(fn `UserConstructionScript`
  (bind (_boxextent_x _boxextent_y _boxextent_z) (`KismetMathLibrary.BreakVector` (`BoxComponent.BoxExtent` (`self.Box`))))
  (`SceneComponent.K2_SetRelativeLocation` (`self.Box`) (`KismetMathLibrary.MakeVector` 0.0 0.0 _boxextent_z) false false))