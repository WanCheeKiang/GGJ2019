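; BP_InteractableObject is an actor that makes an impact noise when it hits something while moving fast enough.
; On Hit, a speed threshold and a DoOnce that resets after a short delay throttle the response.
; It plays ImpactSound at its location with volume mapped from its speed, then calls IncreaseSound on the BP_Player pawn with a value of zero.
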(event `self.ReceiveHit`
  (params (MyComp :type "PrimitiveComponent Object Reference") (Other :type "Actor Object Reference") (OtherComp :type "PrimitiveComponent Object Reference") (bSelfMoved :type Boolean) (HitLocation :type "Vector Structure") (HitNormal :type "Vector Structure") (NormalImpulse :type "Vector Structure") (Hit :type "HitResult Structure (by ref)"))
  (bind _returnvalue (`KismetMathLibrary.VSize` (`self.GetVelocity`)))
  (if (>= _returnvalue 20.0)
    (`/Engine/EditorBlueprintResources/StandardMacros.DoOnce` false :!label _label
      (:`Completed`
        (`|ExecutionSequence`
          (:`then_0`
            (`KismetSystemLibrary.Delay` 0.4)
            (goto _label :!via `Reset`))
          (:`then_1`
            (`GameplayStatics.PlaySoundAtLocation` (`self.ImpactSound`) (`self.K2_GetActorLocation`) (struct) (`KismetMathLibrary.MapRangeClamped` _returnvalue 10.0 100.0 0.0 1.0) 1.0 0.0 null null null)
            (bind _asbp_player (cast `/Game/Blueprints/Player/BP_Player` (`GameplayStatics.GetPlayerPawn` 0)))
            (`/Game/Blueprints/Player/BP_Player.IncreaseSound` _asbp_player 0.0)))))))

(fn `UserConstructionScript`)