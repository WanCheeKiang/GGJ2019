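; Player component that tracks a battery value and is set up to show it on a three-segment HUD battery widget.
; On BeginPlay it caches the player's battery widget and binds to the objective-pickup event; IncreaseBattery refills the value to a fixed cap.
; The drain, segment recolouring and game-over logic are disconnected and never run, and Tick is empty.
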(event `self.ReceiveBeginPlay`
  (bind _asbp_player (cast `/Game/Blueprints/Player/BP_Player` (`self.GetOwner`)))
  (set `self.W_Battery` (`/Game/Blueprints/UMG/WBP_HUD.WBP_BatteryUI` (`/Game/Blueprints/Player/BP_Player.W_HUD` _asbp_player)))
  (add `/Game/Blueprints/Player/BP_Player.OnPickedUpObjective` _asbp_player (`|CreateDelegate` :!event `Increase Battery`)))

(event `Increase Battery`
  (`self.Battery` 30.0))

(event `Battery`
  (params (Batteryvalue :type "Float (double-precision)"))
  ;[1 1 1] Increasing battery value
  (if (> Batteryvalue 0.0)
    (set `self.Battery Value` (`KismetMathLibrary.FMin` (+ (`self.Battery Value`) Batteryvalue) 30.0))))

(event `self.ReceiveTick`
  (params (DeltaSeconds :type "Float (single-precision)")))