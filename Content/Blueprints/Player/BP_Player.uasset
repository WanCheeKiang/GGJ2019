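; Player character for a stealth game, with dashing, objective pickup that applies a speed modifier, and a HUD.
; Dash uses a timeline and raises walk speed, then plays back in reverse at half rate before re-arming.
; Impact noise and light exposure sum into a detection value that triggers game over when full, with light decaying outside lights and sound on a delayed timer.
; Velocity drives the movement audio.
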(event `InputAction|Dash`
  (params (Key :type "Key Structure"))
  (bind _dashing (`self.Dashing`))
  ;[1 1 1] Dashing
  (:`Pressed`
    (if (not (`self.bIsDashing`))
      (set `self.bIsDashing` true)
      (`self.OnDashStarted`)
      (`TimelineComponent.SetPlayRate` (`self.Dashing`) 1.0)
      (set `CharacterMovementComponent.MaxWalkSpeed` (`self.DashMoveSpeed`) (`self.CharacterMovement`))
      (set `self.DashForwardCurrent` (`self.DashForwardSpeed`))
      (set `self.DashHorizontalCurrent` (`self.DashRightModifier`))
      (bind (_direction _dashvalue) (`Timeline|Dashing` :!via `PlayFromStart`)
        (:`Update`
          (set `self.DashValue` _dashvalue))
        (:`Finished`
          (switch `ETimelineDirection` _direction
            (:`Forward`
              (set `self.DashForwardCurrent` 0.0)
              (set `self.DashHorizontalCurrent` 1.0)
              (`KismetSystemLibrary.Delay` 1.0)
              (`TimelineComponent.SetPlayRate` _dashing 0.5)
              (`TimelineComponent.ReverseFromEnd` _dashing)
              (set `CharacterMovementComponent.MaxWalkSpeed` (`self.DefaultMoveSpeed`) (`self.CharacterMovement`)))
            (:`Backward`
              (set `self.bIsDashing` false))))))))

(event `InputAxis|MoveForward`
  (params (AxisValue :type "Float (single-precision)"))
  ;[1 1 1] Movement
  (`self.AddMovementInput` (`KismetMathLibrary.GetForwardVector` (`self.K2_GetActorRotation`)) (`self.GetForwardSpeed`)))

(event `InputAxis|MoveLeft`
  (params (AxisValue :type "Float (single-precision)"))
  ;[1 1 1] Movement
  (`self.AddMovementInput` (`KismetMathLibrary.GetRightVector` (`self.K2_GetActorRotation`)) (`self.GetRightSpeed`)))

(event `self.ReceiveBeginPlay`
  ;[1 1 1] Begin play, setting defaults
  (`self.CreateUI`)
  (set `CharacterMovementComponent.MaxWalkSpeed` (`self.DefaultMoveSpeed`) (`self.CharacterMovement`))
  (`AudioComponent.Play` (`self.RobotMovementCue`) 0.0))

(event `InputAxis|LookUp`
  (params (AxisValue :type "Float (single-precision)"))
  ;[1 1 1] Rotation
  (`self.AddControllerPitchInput` (* AxisValue (`self.DashRightModifier`))))

(event `self.ReceiveHit`
  (params (MyComp :type "PrimitiveComponent Object Reference") (Other :type "Actor Object Reference") (OtherComp :type "PrimitiveComponent Object Reference") (bSelfMoved :type Boolean) (HitLocation :type "Vector Structure") (HitNormal :type "Vector Structure") (NormalImpulse :type "Vector Structure") (Hit :type "HitResult Structure (by ref)"))
  (bind _returnvalue (`KismetMathLibrary.VSize` (`self.GetVelocity`)))
  (`KismetSystemLibrary.PrintString` (`KismetStringLibrary.Conv_DoubleToString` _returnvalue))
  (if (> _returnvalue 100.0)
    (`/Engine/EditorBlueprintResources/StandardMacros.DoOnce` false :!label _label
      (:`Completed`
        (`self.Sound` (* (/ _returnvalue (`self.DashMoveSpeed`)) 0.5))
        (`GameplayStatics.PlaySound2D` "/Game/Art/Audio/Impacts/GGJ19_Cloth_Impact_01.GGJ19_Cloth_Impact_01" 1.0 1.0 0.0 null null)
        (`KismetSystemLibrary.Delay` 0.2)
        (goto _label :!via `Reset`)))))

(event `InputAxis|LookRight`
  (params (AxisValue :type "Float (single-precision)"))
  ;[1 1 1] Rotation
  (`self.AddControllerYawInput` (* AxisValue (`self.DashRightModifier`))))

(event `Sound`
  (params (soundvalue :type "Float (double-precision)"))
  ;[1 0.6482 0.8909] Increasing sound, checking detection value, setting delay timer
  (`KismetSystemLibrary.K2_ClearAndInvalidateTimerHandle` (`self.t_decreaseTimer`))
  (set `self.m_SoundValue` (+ soundvalue (`self.m_SoundValue`)))
  (`self.Check Detection`)
  (`KismetSystemLibrary.RetriggerableDelay` 5.0)
  (bind _returnvalue (`KismetSystemLibrary.K2_SetTimerDelegate` (`|CreateDelegate` :!event `DecreaseSound`) 0.01 true))
  (set `self.t_decreaseTimer` _returnvalue))

(event `self.ReceiveTick`
  (params (DeltaSeconds :type "Float (single-precision)"))
  (bind _robotmovementcue (`self.RobotMovementCue`))
  (bind _returnvalue (/ (`KismetMathLibrary.VSizeXY` (`self.GetVelocity`)) (`self.DashMoveSpeed`)))
  ;[1 0.6958 0] DEBUG PRINTING LIGHT VALUES
  (`|ExecutionSequence`
    (:`then_0`
      (`KismetSystemLibrary.PrintText` (`|FormatText` "Current exposure in light is {EIL}" (`self.lighting Value`)) true true (struct :`G` 0.66 :`B` 1.0 :`A` 1.0) 0.0))
    (:`then_1`
      (`self.Subtract Lighting`))
    (:`then_2`
      (`AudioComponent.SetVolumeMultiplier` _robotmovementcue (`KismetMathLibrary.FInterpTo` (+ _returnvalue 2.0) 1.5 (`GameplayStatics.GetWorldDeltaSeconds`) 10.0)))
    (:`then_3`
      (`AudioComponent.SetPitchMultiplier` _robotmovementcue (`|EaseFunction` "ExpoInOut" _returnvalue 0.5 1.5)))))

(event `DecreaseSound`
  ;[1 0.6482 0.8909] decreasing sound values
  (bind _output_get (set `self.m_SoundValue` (`KismetMathLibrary.FMax` (- (`self.m_SoundValue`) (`self.Sound decrease rate`)))))
  (if (<= _output_get 0.0)
    (`KismetSystemLibrary.K2_ClearAndInvalidateTimerHandle` (`self.t_decreaseTimer`))))

(event `Add Lighting`
  (params (`light amount` :type "Float (double-precision)"))
  ;[0.3069 1 0.379] lighting checking
  (set `self.lighting Value` (`KismetMathLibrary.FClamp` (+ (`self.lighting Value`) `light amount`)))
  (`self.Check Detection`))

(event `Increase Num Lights`
  ;[0.3069 1 0.379] increasing lighting
  (`/Engine/EditorBlueprintResources/StandardMacros.IncrementInt` (`self.Number Lights`)))

(event `Decrease Num Lights`
  ;[0.3069 1 0.379] Decrease lighting numbers
  (set `self.Number Lights` (`KismetMathLibrary.Max` (- (`self.Number Lights`) 1))))

(event `Subtract Lighting`
  ;[0.3069 1 0.379] Subtract lighting value
  (if (<= (`self.Number Lights`) 0)
    (set `self.lighting Value` (`KismetMathLibrary.FClamp` (- (`self.lighting Value`) (`GameplayStatics.GetWorldDeltaSeconds`))))))

(fn `Check Detection`
  (if (>= (`self.Get Detection Value`) 1.0)
    (`/Engine/EditorBlueprintResources/StandardMacros.DoOnce` false
      (:`Completed`
        (bind _asgm_base_game_mode (cast `/Game/Blueprints/Systems/GM_BaseGameMode` (`GameplayStatics.GetGameMode`)))
        (`/Game/Blueprints/Systems/GM_BaseGameMode.GameOver` _asgm_base_game_mode)))))

(fn `CreateUI`
  (bind _returnvalue (`|CreateWidget` "/Game/Blueprints/UMG/WBP_HUD.WBP_HUD_C" (`GameplayStatics.GetPlayerController` 0)))
  (set `self.W_HUD` _returnvalue)
  (`UserWidget.AddToViewport` _returnvalue 0)
  (return))

(fn `Get Detection Value`
  (returns (Detection :type "Float (double-precision)"))
  (return (`KismetMathLibrary.FMin` (+ (`self.m_SoundValue`) (`self.lighting Value`)) 1.0)))

(fn `GetForwardSpeed`
  (returns (Scale :type "Float (double-precision)"))
  (return (* (+ (`self.GetInputAxisValue`) (`self.DashForwardCurrent`)) (`KismetMathLibrary.SelectFloat` (`self.ObjectSpeedModifier`) 1.0 (`self.bHasObjective`)))))

(fn `GetHasObjective`
  (returns (bHasObjective :type Boolean))
  (return (`self.bHasObjective`)))

(fn `GetRightSpeed`
  (returns (Scale :type "Float (double-precision)"))
  (return (* (`self.GetInputAxisValue`) (`self.DashHorizontalCurrent`) (`KismetMathLibrary.SelectFloat` (`self.ObjectSpeedModifier`) 1.0 (`self.bHasObjective`)))))

(fn `IncreaseSound`
  (params (SoundValue :type "Float (double-precision)"))
  (`self.MakeNoise` SoundValue null (`self.K2_GetActorLocation`) 2.0))

(fn `PickupObjective`
  (if (`self.bHasObjective`)
    (return)
    (else
      (set `self.bHasObjective` true)
      (`self.OnPickedUpObjective`)
      (return))))

(fn `UserConstructionScript`)